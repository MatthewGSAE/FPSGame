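; BP_Collectable is a pickup that the player collects by walking into its Box trigger.
; On overlap with the first player's pawn, it increments CollectableCount on BP_FirstPersonPlayerController and prints the new total.
; It then plays a ding sound, spawns an enlarged particle burst at the box's location and destroys itself.
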(event `self.Box.OnComponentBeginOverlap`
  (params (OverlappedComponent :type "PrimitiveComponent Object Reference") (OtherActor :type "Actor Object Reference") (OtherComp :type "PrimitiveComponent Object Reference") (OtherBodyIndex :type Integer) (bFromSweep :type Boolean) (SweepResult :type "HitResult Structure (by ref)"))
  (if (== OtherActor (`GameplayStatics.GetPlayerPawn` 0))
    (bind _asbp_first_person_player_controller (cast `/Game/FirstPerson/Blueprints/BP_FirstPersonPlayerController` (`GameplayStatics.GetPlayerController` 0)))
    (bind _output_get (set `/Game/FirstPerson/Blueprints/BP_FirstPersonPlayerController.CollectableCount` (+ (`/Game/FirstPerson/Blueprints/BP_FirstPersonPlayerController.CollectableCount` _asbp_first_person_player_controller) 1) _asbp_first_person_player_controller))
    (`KismetSystemLibrary.PrintString` (`KismetStringLibrary.Conv_IntToString` _output_get))
    (`GameplayStatics.PlaySound2D` "/Game/ding-126626__1__Cue.ding-126626__1__Cue" 1.0 1.0 0.0 null null)
    (`GameplayStatics.SpawnEmitterAtLocation` "/Game/InfinityBladeEffects/Effects/FX_Monsters/FX_Monster_Ausar/P_AU_Trap_Target.P_AU_Trap_Target" (`SceneComponent.K2_GetComponentLocation` (`self.Box`)) (struct) (20.0 20.0 20.0))
    (`self.K2_DestroyActor`)))

(fn `UserConstructionScript`)