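; AI controller that runs the BT_AI behavior tree and feeds it player perception through the blackboard.
; RunBehaviorTree is called on every Tick, while BeginPlay is empty.
; AI Perception updates for actors tagged "Player" write the IsSeeingPlayer key.
; Both the sensed and lost-stimulus branches set that key to true, so this controller never clears it.
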(event `self.ReceiveTick`
  (params (DeltaSeconds :type "Float (single-precision)"))
  (`self.RunBehaviorTree` "/Game/AI/BT_AI.BT_AI"))

(event `self.AIPerception.OnTargetPerceptionUpdated`
  (params (Actor :type "Actor Object Reference") (Stimulus :type "AIStimulus Structure"))
  (if (`self.ActorHasTag` Actor "Player")
    (if (`.bSuccessfullySensed` (break `AIStimulus` Stimulus))
      (`BlackboardComponent.SetValueAsBool` (`AIBlueprintHelperLibrary.GetBlackboard` null) "IsSeeingPlayer" true)
      (else
        (`BlackboardComponent.SetValueAsBool` (`AIBlueprintHelperLibrary.GetBlackboard` null) "IsSeeingPlayer" true)))))

(fn `UserConstructionScript`)